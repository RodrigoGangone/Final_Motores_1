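; Interactive door that the player opens with the E key while standing in its trigger Box.
; Box overlaps with BP_ThirdPersonCharacter toggle input on the door and show or remove the WBP_InteractionDoor prompt.
; E drives a FlipFlop that plays or reverses the AbrirPuerta timeline, lerping the Arrow's yaw between closed and open.
; The timeline update also disables Box collision, which is never re-enabled here.
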(event `Key|E`
  (params (Key :type "Key Structure"))
  ;[0 0.1874 1] Que ocurre al presionar "E"
  (:`Pressed`
    (`/Engine/EditorBlueprintResources/StandardMacros.FlipFlop`
      (:`A`
        (bind (_direction _animpuerta) (`Timeline|Abrir Puerta` :!label _label)
          (:`Update`
            ;;[0.2116 0.3876 1] Rotar la puerta en eje "Z"
            (`SceneComponent.K2_SetRelativeRotation` (`self.Arrow`) (`KismetMathLibrary.MakeRotator` 0.0 0.0 (`KismetMathLibrary.Lerp` (`self.PuertaCerrada`) (`self.PuertaAbierta`) _animpuerta)) false false)
            ;;[1 0.07409 0.3366] Deshabilito el Box una vez presionado el Input
            (`PrimitiveComponent.SetCollisionEnabled` (`self.Box`) "NoCollision"))))
      (:`B`
        (goto _label :!via `Reverse`)))))

(event `self.Box.OnComponentBeginOverlap`
  (params (OverlappedComponent :type "PrimitiveComponent Object Reference") (OtherActor :type "Actor Object Reference") (OtherComp :type "PrimitiveComponent Object Reference") (OtherBodyIndex :type Integer) (bFromSweep :type Boolean) (SweepResult :type "HitResult Structure (by ref)"))
  ;[0.1705 1 0.5122] Entro algo en la Box
  ;[0.1705 1 0.5122] El personaje entro en la Box
  (cast `/Game/Blueprints/BP_ThirdPersonCharacter` OtherActor)
  (`self.EnableInput` (`GameplayStatics.GetPlayerController` 0))
  (bind _returnvalue (`|CreateWidget` "/Game/WidgetBlueprints/WBP_InteractionDoor.WBP_InteractionDoor_C"))
  (`UserWidget.AddToViewport` _returnvalue 0))

(event `self.Box.OnComponentEndOverlap`
  (params (OverlappedComponent :type "PrimitiveComponent Object Reference") (OtherActor :type "Actor Object Reference") (OtherComp :type "PrimitiveComponent Object Reference") (OtherBodyIndex :type Integer))
  ;[1 0.2376 0.2077] Salio algo en la Box
  ;[1 0.2376 0.2077] El personaje salio de la Box
  (cast `/Game/Blueprints/BP_ThirdPersonCharacter` OtherActor)
  (`self.DisableInput` (`GameplayStatics.GetPlayerController` 0))
  (`Widget.RemoveFromParent` (stale `self.Box.OnComponentBeginOverlap` _returnvalue)))

(fn `UserConstructionScript`)